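; WaterVolume is a configurable box of ocean water with a surface and sound, set up entirely in the construction script.
; Extent sizes the box, scales and raises the surface mesh, and drives the box-shaped attenuation of the audio component.
; A dynamic instance of the ocean material receives the exposed speed, scale, displacement, tessellation and wave amplification settings.
; The event graph holds no active logic.
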(event EventBeginPlay)

(event Collision|EventActorBeginOverlap
  (params (OtherActor :type Actor%20Object%20Reference)))

(event EventTick
  (params (DeltaSeconds :type Float%20%28single-precision%29)))

(fn ConstructionScript
  (bind _extent (Variables|Default|GetExtent))
  (bind _watersurface (Variables|Default|GetWaterSurface))
  (bind _008 (Variables|Default|Get008))
  (bind _returnvalue (/ _extent 5e+01))
  (Components|Box|SetBoxExtent (Variables|Default|GetBox) _extent true)
  (Transformation|SetRelativeScale3D _watersurface _returnvalue)
  (Transformation|AddLocalOffset _watersurface (Math|Vector|MakeVector 0.0 0.0 (.Z (Math|Vector|BreakVector _extent))) false false)
  (bind _returnvalue_2 (Rendering|Material|CreateDynamicMaterialInstance "/Game/WaterPlane/Ocean/Materials/M_OceanWater_1_Inst.M_OceanWater_1_Inst" "None" :!class /Script/Engine.KismetMaterialLibrary))
  (bind _output_get (Variables|Default|SetWaterMaterial _returnvalue_2))
  (Rendering|Material|SetMaterial (Variables|Default|GetWaterSurface) 0 _output_get)
  (CallFunction|SetWaterMaterialParameters)
  (Audio|Components|Audio|AdjustAttenuation _008 (Utilities|Struct|MakeSoundAttenuationSettings true true false false false false false true false false false false "SPATIALIZATION_Default" 0.0 "Linear" "ECC_Visibility" "Linear" "Linear" 0.0 2e+02 3e+03 6e+03 "(EditorCurveData=(Keys=,DefaultValue=340282346638528859811704183484516925440.000000,PreInfinityExtrap=RCCE_Constant,PostInfinityExtrap=RCCE_Constant),ExternalCurve=None)" "(EditorCurveData=(Keys=,DefaultValue=340282346638528859811704183484516925440.000000,PreInfinityExtrap=RCCE_Constant,PostInfinityExtrap=RCCE_Constant),ExternalCurve=None)" 2e+04 2e+04 0.0 0.0 3e+01 6e+01 1.0 1.0 1.0 1.0 1.0 1.0 1.0 1.0 2e+04 1.0 0.1 0.3 0.95 4e+02 4e+03 0.0 "(EditorCurveData=(Keys=,DefaultValue=340282346638528859811704183484516925440.000000,PreInfinityExtrap=RCCE_Constant,PostInfinityExtrap=RCCE_Constant),ExternalCurve=None)" 0 1.0 1.0 4e+02 4e+03 1.0 "(EditorCurveData=(Keys=,DefaultValue=340282346638528859811704183484516925440.000000,PreInfinityExtrap=RCCE_Constant,PostInfinityExtrap=RCCE_Constant),ExternalCurve=None)" "(SpatializationPluginSettingsArray=,OcclusionPluginSettingsArray=,ReverbPluginSettingsArray=)" "Linear" (Utilities|Enum|LiteralenumEAttenuationShape "Box") (Math|Float|MakeLiteralFloat 1e+01) "Continues" _returnvalue 0.0 (Math|Float|MakeLiteralFloat 1e+01)))
  (Audio|Components|Audio|AdjustVolume _008 0.0 2e+02 "Linear" :!class /Script/Engine.AudioComponent))

(fn SetWaterMaterialParameters
  (bind _watermaterial (Variables|Default|GetWaterMaterial))
  (Rendering|Material|SetScalarParameterValue _watermaterial "WaterSpeed" (Variables|Default|GetOverall%20Water%20Speed) :!class /Script/Engine.MaterialInstanceDynamic)
  (Rendering|Material|SetScalarParameterValue _watermaterial "WaterScale" (Variables|Default|GetOverall%20Water%20Scale) :!class /Script/Engine.MaterialInstanceDynamic)
  (Rendering|Material|SetScalarParameterValue _watermaterial "Displacement" (Variables|Default|GetDisplacement) :!class /Script/Engine.MaterialInstanceDynamic)
  (Rendering|Material|SetScalarParameterValue _watermaterial "Tesselation" (Variables|Default|GetTesselation%20Factor) :!class /Script/Engine.MaterialInstanceDynamic)
  (Rendering|Material|SetScalarParameterValue _watermaterial "Large Wave Amplify" (Variables|Default|GetAmplify%20Large%20Normals) :!class /Script/Engine.MaterialInstanceDynamic)
  (Rendering|Material|SetScalarParameterValue _watermaterial "Small Wave Amplify" (Variables|Default|GetAmplify%20Small%20Normals) :!class /Script/Engine.MaterialInstanceDynamic))